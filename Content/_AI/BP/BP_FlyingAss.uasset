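; BP_FlyingAss is an AI-driven flying pawn that runs BT_FlyToPos and yaws toward the first-person player every tick.
; It supplies goals beside the player or at random spots before the camera, plus the player's idle and moving states.
; ToggleFlapping switches between floating pawn movement and gravity-driven flapping through FlappyComponent.
; GetFlapState returns the inverse of the Flap flag, and random offsets use world axes.
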(event EventTick
  (params (DeltaSeconds :type Float%20%28single-precision%29))
  (CallFunction|LookatPlayer))

(event EventBeginPlay
  (bind _asbp_aicontroller (Utilities|Casting|CastToBP_AIController (Pawn|GetController)))
  (bind _output_get (Variables|Default|SetAC _asbp_aicontroller))
  (AI|RunBehaviorTree _output_get "/Game/_AI/BehaviorTree/BT_FlyToPos.BT_FlyToPos")
  (bind _asfirst_person_character (Utilities|Casting|CastToFirstPersonCharacter (Game|Player|GetPlayerPawn 0)))
  (Variables|Default|SetChar _asfirst_person_character))

(fn ConstructionScript)

(fn FindRandomSpotinFrontOfPlayer
  (bind _char (Variables|Default|GetChar))
  (bind _firstpersoncamera (Variables|/Game/FirstPersonBP/Blueprints/FirstPersonCharacter.FirstPersonCharacter_C|GetFirstPersonCamera _char))
  (bind _returnvalue (Math|Vector|GetForwardVector _firstpersoncamera))
  (bind _returnvalue_2 (Transformation|GetWorldLocation _firstpersoncamera))
  (bind _returnvalue_3 (* _returnvalue 5e+01))
  (bind _returnvalue_4 (+ _returnvalue_2 _returnvalue_3))
  (bind (_x _y _z) (Math|Vector|BreakVector _returnvalue_4))
  (return (Math|Vector|MakeVector _x (+ _y (Math|Random|RandomFloatinRange -35.0 35.0)) (+ _z (Math|Random|RandomFloatinRange -16.0 15.0)))))

(fn LookatPlayer
  (Transformation|SetActorRotation (Math|Rotator|MakeRotator 0.0 0.0 (- (.Yaw (Math|Rotator|BreakRotator (Math|Rotator|FindLookatRotation (Transformation|GetActorLocation) (Transformation|GetActorLocation (Variables|Default|GetChar))))) 9e+01))))

(fn ToggleFlapping
  (params (bIsFlap :type Boolean))
  (bind _self self)
  (bind _floatingpawnmovement (Variables|BP_FlyingAss_C|GetFloatingPawnMovement _self))
  (bind _capsule (Variables|BP_FlyingAss_C|GetCapsule _self))
  (bind _flappycomponent (Variables|BP_FlyingAss_C|GetFlappyComponent _self))
  (if bIsFlap
    (Components|Activation|Deactivate _floatingpawnmovement)
    (Variables|/Game/_Termanteus/Component/FlappyComponent.FlappyComponent_C|SetbFlap _flappycomponent true)
    (Physics|SetEnableGravity _capsule true)
    (else
      (Variables|/Game/_Termanteus/Component/FlappyComponent.FlappyComponent_C|SetbFlap _flappycomponent false)
      (Physics|SetEnableGravity _capsule false)
      (Components|Activation|Activate _floatingpawnmovement false))))

(fn GetFlapState
  (return (not (Variables|/Game/_Termanteus/Component/FlappyComponent.FlappyComponent_C|GetbFlap (Variables|Default|GetFlappyComponent)))))

(fn GetFlightGoal
  (bind _char (Variables|Default|GetChar))
  (return (+ (+ (+ (* (Transformation|GetActorRightVector _char) 1.2e+02) (Transformation|GetActorLocation _char)) (* (Transformation|GetActorForwardVector _char) 6e+01)) "0, 0,90.000000")))

(fn GetGoalActor
  (return (Game|Player|GetPlayerPawn 0)))

(fn GetIdleState
  (return (Variables|/Game/FirstPersonBP/Blueprints/FirstPersonCharacter.FirstPersonCharacter_C|GetbIsIdle (Variables|Default|GetChar))))

(fn GetMoveState
  (return (Variables|/Game/FirstPersonBP/Blueprints/FirstPersonCharacter.FirstPersonCharacter_C|GetbIsMoving (Variables|Default|GetChar))))